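; BP_PlatfomerChar is a 2D sprite platformer character Blueprint whose only active logic is its defeat sequence.
; A one-shot Defeat event disables capsule collision, releases the movement plane constraint and calls LaunchDefeat to throw the character upward and along Y, scaled by DefeatLaunchUp.
; It also jumps the animation instance to its defeated node and raises the sprite's translucent sort priority.
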(event `Defeat`
  (if (not (`self.IsDefeated`))
    (set `self.IsDefeated` true)
    (`PrimitiveComponent.SetCollisionEnabled` (`self.CapsuleComponent`) "NoCollision")
    (`MovementComponent.SetPlaneConstraintEnabled` (`self.CharacterMovement`) false)
    (`self.LaunchDefeat`)
    (`PaperZDAnimInstance.JumpToNode` (`self.AnimInstance`) "JumpDefeated" "None")
    (`PrimitiveComponent.SetTranslucentSortPriority` (`self.Sprite`) 100)))

(fn `LaunchDefeat`
  (`self.LaunchCharacter` (* (0.0 0.3 1.0) (`self.DefeatLaunchUp`)) true true))

(fn `UserConstructionScript`)