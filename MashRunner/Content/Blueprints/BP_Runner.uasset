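; BP_Runner is a 2D flipbook runner character that constantly moves along +X, with speed driven by left and right power presses.
; Each press raises MaxWalkSpeed through a velocity-sampled curve and records LastInput, which does not gate the boost.
; Tick decays speed through another curve, switches idle/run flipbooks and scales run playback by velocity.
; Footsteps fire once on set run frames; PlayStepSound duplicates this inline logic but is never called.
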(event `self.ReceiveBeginPlay`
  (bind `_as플레이어_컨트롤러` (cast `PlayerController` (`self.GetController`)))
  (`EnhancedInputSubsystemInterface.AddMappingContext` (pcsubsystem `EnhancedInputLocalPlayerSubsystem` `_as플레이어_컨트롤러`) "/Game/Input/IMC_Runner.IMC_Runner" 0 (struct)))

(event `self.ReceiveTick`
  (params (DeltaSeconds :type "Float (single-precision)"))
  (bind _returnvalue (`PaperFlipbookComponent.GetPlaybackPositionInFrames` (`self.Sprite`)))
  (`self.AddMovementInput` (1.0 0.0 0.0))
  (`self.SpeedDown`)
  (`self.UpdateFlipbook`)
  (`self.SetPlayRate`)
  (if (== (`PaperFlipbookComponent.GetFlipbook` (`self.Sprite`)) "/Game/PaperAssets/Runner/FB_Runner_Run.FB_Runner_Run")
    (if (or (== _returnvalue 1) (== _returnvalue 5))
      (`/Engine/EditorBlueprintResources/StandardMacros.DoOnce` false :!label _label
        (:`Completed`
          (`GameplayStatics.PlaySound2D` "/Game/Sounds/Footsteps/Cue_Footstep.Cue_Footstep" 1.0 1.0 0.0 null null)))
      (else
        (goto _label :!via `Reset`)))))

(event `EnhancedInput|/Game/Input/Actions/IA_PowerLeft`
  (params (ActionValue :type Boolean) (ElapsedSeconds :type "Float (double-precision)") (TriggeredSeconds :type "Float (double-precision)") (InputAction :type "InputAction Object Reference" :default "/Game/Input/Actions/IA_PowerLeft.IA_PowerLeft"))
  (:`Started`
    (`self.SpeedUp`)
    (if (`|EnumInequality` (`self.LastInput`) "NewEnumerator1")
      (set `self.LastInput` "NewEnumerator1"))))

(event `EnhancedInput|/Game/Input/Actions/IA_PowerRight`
  (params (ActionValue :type Boolean) (ElapsedSeconds :type "Float (double-precision)") (TriggeredSeconds :type "Float (double-precision)") (InputAction :type "InputAction Object Reference" :default "/Game/Input/Actions/IA_PowerRight.IA_PowerRight"))
  (:`Started`
    (`self.SpeedUp`)
    (if (`|EnumInequality` (`self.LastInput`) "NewEnumerator2")
      (set `self.LastInput` "NewEnumerator2"))))

(fn `PlayStepSound`
  (bind _returnvalue (`PaperFlipbookComponent.GetPlaybackPositionInFrames` (`self.Sprite`)))
  (if (== (`PaperFlipbookComponent.GetFlipbook` (`self.Sprite`)) "/Game/PaperAssets/Runner/FB_Runner_Run.FB_Runner_Run")
    (if (or (== _returnvalue 1) (== _returnvalue 5))
      (`/Engine/EditorBlueprintResources/StandardMacros.DoOnce` false :!label _label
        (:`Completed`
          (`GameplayStatics.PlaySound2D` "/Game/Sounds/Footsteps/Cue_Footstep.Cue_Footstep" 1.0 1.0 0.0 null null)))
      (else
        (goto _label :!via `Reset`)))))

(fn `SetPlayRate`
  (bind _sprite (`self.Sprite`))
  (if (== (`PaperFlipbookComponent.GetFlipbook` (`self.Sprite`)) "/Game/PaperAssets/Runner/FB_Runner_Run.FB_Runner_Run")
    (`PaperFlipbookComponent.SetPlayRate` _sprite (/ (`KismetMathLibrary.VSize` (`MovementComponent.Velocity` (`self.CharacterMovement`))) (`self.MaxSpeed`)))
    (else
      (`PaperFlipbookComponent.SetPlayRate` _sprite 1.0))))

(fn `SpeedDown`
  (set `CharacterMovementComponent.MaxWalkSpeed` (`KismetMathLibrary.FMax` (- (`CharacterMovementComponent.MaxWalkSpeed` (`self.CharacterMovement`)) (* (`GameplayStatics.GetWorldDeltaSeconds`) (* (`self.SlowMultiplier`) (`CurveFloat.GetFloatValue` (`self.SpeedDownCurve`) (`KismetMathLibrary.VSize` (`MovementComponent.Velocity` (`self.CharacterMovement`)))))))) (`self.CharacterMovement`)))

(fn `SpeedUp`
  (set `CharacterMovementComponent.MaxWalkSpeed` (`KismetMathLibrary.FClamp` (+ (`CharacterMovementComponent.MaxWalkSpeed` (`self.CharacterMovement`)) (* (`self.StepSpeed`) (`CurveFloat.GetFloatValue` (`self.SpeedUpCurve`) (`KismetMathLibrary.VSize` (`MovementComponent.Velocity` (`self.CharacterMovement`)))))) 0.0 (`self.MaxSpeed`)) (`self.CharacterMovement`)))

(fn `UpdateFlipbook`
  (`PaperFlipbookComponent.SetFlipbook` (`self.Sprite`) (select `bool` (> (`KismetMathLibrary.VSize` (`MovementComponent.Velocity` (`self.CharacterMovement`))) 0.0) :`false` "/Game/PaperAssets/Runner/FB_Runner_Idle.FB_Runner_Idle" :`true` "/Game/PaperAssets/Runner/FB_Runner_Run.FB_Runner_Run" :!type "PaperFlipbook Object Reference")))

(fn `UserConstructionScript`)